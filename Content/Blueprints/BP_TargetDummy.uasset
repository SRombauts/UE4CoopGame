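; BP_TargetDummy is a test target that visualizes incoming damage for debugging.
; Point damage draws a red debug sphere at the hit location and a label pairing the hit's physical surface type (Flesh, Vulnerable or unknown) with the damage amount.
; Radial damage only prints the received amount to the screen.
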(event `self.ReceivePointDamage`
  (params (Damage :type "Float (single-precision)") (DamageType :type "DamageType Object Reference") (HitLocation :type "Vector Structure") (HitNormal :type "Vector Structure") (HitComponent :type "PrimitiveComponent Object Reference") (BoneName :type Name) (ShotFromDirection :type "Vector Structure") (InstigatedBy :type "Controller Object Reference") (DamageCauser :type "Actor Object Reference") (HitInfo :type "HitResult Structure (by ref)"))
  (`KismetSystemLibrary.DrawDebugSphere` HitLocation 5.0 12 (struct :`R` 1.0 :`A` 1.0) (`self.Duration`) 1.0)
  (`KismetSystemLibrary.DrawDebugString` HitLocation (`KismetStringLibrary.Concat_StrStr` (select `EPhysicalSurface` (`GameplayStatics.GetSurfaceType` HitInfo) :`SurfaceType_Default` "?" :`SurfaceType1` "Flesh" :`SurfaceType2` "Vulnerable") ": " (`KismetStringLibrary.Conv_DoubleToString` Damage)) null (struct :`R` 1.0 :`G` 1.0 :`B` 1.0 :`A` 1.0) (`self.Duration`)))

(event `self.ReceiveRadialDamage`
  (params (DamageReceived :type "Float (single-precision)") (DamageType :type "DamageType Object Reference") (Origin :type "Vector Structure") (HitInfo :type "HitResult Structure (by ref)") (InstigatedBy :type "Controller Object Reference") (DamageCauser :type "Actor Object Reference"))
  (`KismetSystemLibrary.PrintString` (`KismetStringLibrary.Conv_DoubleToString` DamageReceived)))

(fn `UserConstructionScript`)